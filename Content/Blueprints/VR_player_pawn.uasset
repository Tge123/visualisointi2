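; VR player pawn that turns its camera with device motion sensors and tracks the actor being looked at.
; Shortly after BeginPlay it sets the starting camera pitch from the gravity reading.
; The rotation axis event then adds the sensor rotation rate to the camera's local pitch and yaw.
; Each tick a debug-drawn line trace from the camera stores the hit actor in MihinOsutaan.
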(event EventBeginPlay
  (bind _returnvalue (Game|GetPlayerController 0))
  ;[1 1 1] Asetetaan kamera oikeaan kulmaan
  (Input|EnableInput _returnvalue)
  (Utilities|FlowControl|Delay 0.1)
  (Transformation|SetRelativeRotation (Variables|Default|GetCamera) (Math|Rotator|MakeRotator 0.0 (* (- 9e+01 (* (* (.X (Math|Vector|BreakVector (.Gravity (Class|PlayerController|GetInputMotionState _returnvalue)))) 1e+01) 0.9)) -1.0) (.Pitch (Math|Rotator|BreakRotator (Transformation|GetWorldRotation (Variables|Default|GetCamera))))) false false))

(event EventTick
  (params (DeltaSeconds :type Float%20%28single-precision%29))
  (bind _camera (Variables|Default|GetCamera))
  (bind _returnvalue (Transformation|GetWorldLocation _camera))
  ;[1 1 1] Mihin katsotaan
  (bind _outhit (Collision|LineTraceByChannel _returnvalue (+ (* (Math|Vector|GetForwardVector _camera) 6e+03) _returnvalue) "TraceTypeQuery2" false 0 "ForOneFrame" true "(R=0.000000,G=0.000000,B=0.000000,A=0.000000)" "(R=1.000000,G=0.000000,B=0.000000,A=1.000000)"))
  (Variables|Default|Setmihin_osutaan (.HitActor (Collision|BreakHitResult _outhit))))

(event Input|AxisEvents|InputAxisrotation
  (params (AxisValue :type Float%20%28single-precision%29))
  (bind _returnvalue (Game|GetPlayerController 0))
  (bind (_tilt _rotationrate _gravity) (Class|PlayerController|GetInputMotionState _returnvalue))
  (bind (_x _y) (Math|Vector|BreakVector _rotationrate))
  ;[1 1 1] Katselu
  (Transformation|AddLocalRotation (Variables|Default|GetCamera) (Math|Rotator|MakeRotator 0.0 (* _x -1.0) (* _y -1.0)) false false))

(fn ConstructionScript)